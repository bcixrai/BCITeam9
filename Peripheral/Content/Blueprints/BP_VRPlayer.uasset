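; BP_VRPlayer is the VR player, with setup and a helper for finding grabbable objects.
; On BeginPlay, if a headset is enabled, it sets floor tracking, pixel density and player input.
; GetGrabComponentsNearMotionController sphere-traces physics bodies at a controller and returns the nearest GrabComponent on the single hit actor, using squared distances.
; The helper prints debug messages and is not called within this file.
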(event EventBeginPlay
  (if (Class|HeadMountedDisplayFunctionLibrary|IsHeadMountedDisplayEnabled)
    (Class|HeadMountedDisplayFunctionLibrary|SetTrackingOrigin "Floor")
    (Development|ExecuteConsoleCommand "vr.PixelDensity 1.0" 0)
    (Input|EnableInput (Game|GetPlayerController 0))))

(event Collision|EventActorBeginOverlap
  (params (OtherActor :type Actor%20Object%20Reference)))

(event EventTick
  (params (DeltaSeconds :type Float%20%28single-precision%29)))

(fn ConstructionScript)

(fn GetGrabComponentsNearMotionController
  (params (MotionController :type Motion%20Controller%20Component%20Object%20Reference))
  (Development|PrintString "Grab Near Motion")
  (Utilities|FlowControl|Sequence
    (:then_0
      ;[1 1 1] Get Grab Position and Sphere trace
      (bind _output_get (LocalVariables|SetLocalGripPosition (Transformation|GetWorldLocation MotionController)))
      (bind (_outhit _returnvalue) (Collision|SphereTraceForObjects _output_get _output_get (Variables|Default|GetGrabRadiusFromGripPosition) (Utilities|Array|MakeArray "ObjectTypeQuery4") false 0 "None"))
      (if _returnvalue
        ;[1 1 1] Does the actors hit have a grab component
        (if (> (Utilities|Array|Length (Actor|GetComponentsByClass (.HitActor (Collision|BreakHitResult _outhit)) "/Script/Peripheral.GrabComponent")) 0)
          (bind _output_get_2 (LocalVariables|SetLocalComponents (Actor|GetComponentsByClass (.HitActor (Collision|BreakHitResult _outhit)) "/Script/Peripheral.GrabComponent")))
          (for _array_element _output_get_2
            (if (<= (Math|Vector|VectorLengthSquared (- (Transformation|GetWorldLocation _array_element) (LocalVariables|GetLocalGripPosition))) (LocalVariables|GetLocalNearestComponentDistance))
              (LocalVariables|SetLocalNearestComponentDistance (Math|Vector|VectorLengthSquared (- (Transformation|GetWorldLocation _array_element) (LocalVariables|GetLocalGripPosition))))
              (LocalVariables|SetLocalNearestGrabComponent _array_element))))
        (else
          (Development|PrintString "No Objects Sphere Traced" true true "(R=1.000000,G=0.050593,B=0.000000,A=1.000000)"))))
    (:then_1
      ;[1 1 1] If a nearby has been found this will be the nearest
      (return (LocalVariables|GetLocalNearestGrabComponent)))))