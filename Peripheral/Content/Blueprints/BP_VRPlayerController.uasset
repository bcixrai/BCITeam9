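; VR player controller that positions the player at level start and handles pause and animal-reaction keys.
; On BeginPlay it moves and rotates the VRPlayer pawn to the first BP_PlayerStartLocationActor found, printing a notice when several exist.
; Escape and pipe keys call Pause on the GI_Peripheral game instance.
; Keys 1 and 2 trigger SAD or HAPPY InteractWithPlayer reactions on every Animal in the world.
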(event EventBeginPlay
  (Utilities|FlowControl|Sequence
    (:then_0
      ;[1 1 1] Change player location
      (bind _outactors (Actor|GetAllActorsOfClass "/Game/Blueprints/BP_PlayerStartLocationActor.BP_PlayerStartLocationActor_C"))
      (if (> (Utilities|Array|Length _outactors) 1)
        (Development|PrintString (Utilities|String|Append "PC : Found " (Utilities|String|ToString(Integer) (Utilities|Array|Length _outactors)) " start locations, using 0th")))
      (bind _asvrplayer (Utilities|Casting|CastToVRPlayer (Game|Player|GetPlayerPawn 0))
        (:then
          (Transformation|SetActorLocation _asvrplayer (Transformation|GetActorLocation (Utilities|Array|Get(acopy) _outactors)) false false)
          (Transformation|SetActorRotation _asvrplayer (Transformation|GetActorRotation (Utilities|Array|Get(acopy) _outactors))))
        (:CastFailed
          (Development|PrintString "PC : No Player" true true "(R=1.000000,G=0.027538,B=0.000000,A=1.000000)"))))))

(event EventTick
  (params (DeltaSeconds :type Float%20%28single-precision%29)))

(event Input|KeyboardEvents||
  (params (Key :type Key%20Structure :default "None"))
  ;[1 1 1] Pausing
  (:Pressed
    (bind _asgi_peripheral (Utilities|Casting|CastToGI_Peripheral (Game|GetGameInstance)))
    (Default|Pause _asgi_peripheral)))

(event Input|KeyboardEvents|1
  (params (Key :type Key%20Structure :default "None"))
  (:Pressed
    (bind _outactors (Actor|GetAllActorsOfClass "/Script/Peripheral.Animal"))
    (for _array_element _outactors
      (Class|Animal|InteractwithPlayer _array_element 0 "SAD"))))

(event Input|KeyboardEvents|2
  (params (Key :type Key%20Structure :default "None"))
  (:Pressed
    (bind _outactors (Actor|GetAllActorsOfClass "/Script/Peripheral.Animal"))
    (for _array_element _outactors
      (Class|Animal|InteractwithPlayer _array_element 0 "HAPPY"))))

(event Input|KeyboardEvents|Escape
  (params (Key :type Key%20Structure :default "None"))
  ;[1 1 1] Pausing
  (:Pressed
    (bind _asgi_peripheral (Utilities|Casting|CastToGI_Peripheral (Game|GetGameInstance)))
    (Default|Pause _asgi_peripheral)))

(fn ConstructionScript)