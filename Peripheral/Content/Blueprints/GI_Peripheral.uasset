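; Game instance for the Peripheral project that registers the selectable user profiles and the game's levels at startup.
; On Init, a sequence adds two hardcoded profiles, then the lobby, the activity maps and the main menu.
; Each level entry pairs a title, description, map name and thumbnail through AddLevel, with many images appearing to be placeholder textures.
; An unconnected test-level entry never runs.
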(event EventInit
  (Utilities|FlowControl|Sequence
    (:then_0
      ;[1 1 1] Profiles
      (Class|PeripheralGameInstance|AddProfile (Utilities|Struct|MakeProfile "Adam" "Adam" "Very bald" "/Game/Assets_+_Textures/Assets/Library/Books_and_drinks/Var3/Redstem_Colocasia_4K_Albedo.Redstem_Colocasia_4K_Albedo"))
      (Class|PeripheralGameInstance|AddProfile (Utilities|Struct|MakeProfile "Santa" "Adam" "Sees you when you're sleeping" "/Game/Assets_+_Textures/Textures/SHELF_/shelf_metal_handle_OcclusionRoughnessMetallic.shelf_metal_handle_OcclusionRoughnessMetallic")))
    (:then_1
      ;[1 1 1] Lobby Map
      (Class|PeripheralGameInstance|AddLevel (Utilities|Struct|MakePeripheralLevel "Lobby" "Lobby" "M_Lobby" "/Game/Assets_+_Textures/Textures/FIREPLACE/Fireplace_Fireplace2_OcclusionRoughnessMetallic.Fireplace_Fireplace2_OcclusionRoughnessMetallic")))
    (:then_2
      ;[1 1 1] Level Maps
      (Class|PeripheralGameInstance|AddLevel (Utilities|Struct|MakePeripheralLevel "Animal Play" "Play with an animal" "M_AnimalPetting" "/Game/Levels/AnimalPetting/Depositphotos_4953129_original-1-256x256.Depositphotos_4953129_original-1-256x256"))
      (Class|PeripheralGameInstance|AddLevel (Utilities|Struct|MakePeripheralLevel "Wood Stacking" "Relaxing wood stacking" "M_WoodStacking" "/Game/Levels/WoodStacking/StackOfWoodPhoto.StackOfWoodPhoto"))
      (Class|PeripheralGameInstance|AddLevel (Utilities|Struct|MakePeripheralLevel "Music Box" "Music Level" "M_MusicBox" "/Game/Assets_+_Textures/Textures/CHAIR/ArmChair_ArmChair_Wood_OcclusionRoughnessMetallic.ArmChair_ArmChair_Wood_OcclusionRoughnessMetallic"))
      (Class|PeripheralGameInstance|AddLevel (Utilities|Struct|MakePeripheralLevel "Painting" "Paint in VR or with Brain" "M_Painting" "/Game/Assets_+_Textures/Textures/BOOK/Green/book_books_OcclusionRoughnessMetallic.book_books_OcclusionRoughnessMetallic")))
    (:then_3
      ;[1 1 1] Extras
      (Class|PeripheralGameInstance|AddLevel (Utilities|Struct|MakePeripheralLevel "Main Menu" "The main menu" "M_MainMenu" "/Game/Assets_+_Textures/Textures/BOOK/books_texture3011.books_texture3011")))))